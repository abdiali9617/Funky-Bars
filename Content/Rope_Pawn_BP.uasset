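; Rope pawn with two independently controlled physics spheres acting as hands that grab "Bar"-tagged components, apparently for climbing or swinging.
; Move axes offset each sphere, or disable its physics to pin it while grabbing; lift input suspends gravity and grabs on bar contact.
; A free sphere gets upward force while the other grips, the left also before its first grab.
; Overlaps swap materials, and the spring arm tracks the spheres' and cone's average X.
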(event OnComponentBeginOverlap(Sphere1)
  (params (OverlappedComponent :type Primitive%20Component%20Object%20Reference) (OtherActor :type Actor%20Object%20Reference) (OtherComp :type Primitive%20Component%20Object%20Reference) (OtherBodyIndex :type Integer) (bFromSweep :type Boolean) (SweepResult :type Hit%20Result%20Structure%20%28by%20ref%29))
  ;[1 1 1] Check for 'CanMoveL'
  (Variables|Default|SetisTouchingBar_L (Components|ComponentHasTag OtherComp "Bar"))
  (Rendering|Material|SetMaterial (Variables|Default|GetSphere1) 0 "/Game/StarterContent/Materials/M_Tech_Hex_Tile_Pulse.M_Tech_Hex_Tile_Pulse"))

(event OnComponentEndOverlap(Sphere1)
  (params (OverlappedComponent :type Primitive%20Component%20Object%20Reference) (OtherActor :type Actor%20Object%20Reference) (OtherComp :type Primitive%20Component%20Object%20Reference) (OtherBodyIndex :type Integer))
  ;[1 1 1] Check for 'CanMoveL'
  (Variables|Default|SetisTouchingBar_L (not (Components|ComponentHasTag OtherComp "Bar")))
  (Rendering|Material|SetMaterial (Variables|Default|GetSphere1) 0 "/Game/StarterContent/Materials/M_Wood_Oak.M_Wood_Oak"))

(event OnComponentBeginOverlap(Sphere)
  (params (OverlappedComponent :type Primitive%20Component%20Object%20Reference) (OtherActor :type Actor%20Object%20Reference) (OtherComp :type Primitive%20Component%20Object%20Reference) (OtherBodyIndex :type Integer) (bFromSweep :type Boolean) (SweepResult :type Hit%20Result%20Structure%20%28by%20ref%29))
  ;[1 1 1] Check for 'CanMoveR'
  (Variables|Default|SetisTouchingBar_R (Components|ComponentHasTag OtherComp "Bar"))
  (Rendering|Material|SetMaterial (Variables|Default|GetSphere) 0 "/Game/StarterContent/Materials/M_Tech_Hex_Tile_Pulse.M_Tech_Hex_Tile_Pulse"))

(event OnComponentEndOverlap(Sphere)
  (params (OverlappedComponent :type Primitive%20Component%20Object%20Reference) (OtherActor :type Actor%20Object%20Reference) (OtherComp :type Primitive%20Component%20Object%20Reference) (OtherBodyIndex :type Integer))
  ;[1 1 1] Check for 'CanMoveR'
  (Variables|Default|SetisTouchingBar_R (not (Components|ComponentHasTag OtherComp "Bar")))
  (Rendering|Material|SetMaterial (Variables|Default|GetSphere) 0 "/Game/StarterContent/Materials/M_Wood_Oak.M_Wood_Oak"))

(event EventTick
  (params (DeltaSeconds :type Float%20%28single-precision%29))
  ;[1 1 1] Camera Movement
  (Transformation|SetWorldLocation (Variables|Default|GetSpringArm) (Math|Vector|MakeVector (.X (Math|Vector|BreakVector (Math|Vector|GetVectorArrayAverage (Utilities|Array|MakeArray (Transformation|GetWorldLocation (Variables|Default|GetSphere)) (Transformation|GetWorldLocation (Variables|Default|GetSphere1)) (Transformation|GetWorldLocation (Variables|Default|GetCone)))))) 8.4e+02 2e+02) false false))

(event Input|ActionEvents|InputActionLift_L_Action
  (params (Key :type Key%20Structure :default "None"))
  (bind _sphere1 (Variables|Default|GetSphere1))
  (:Pressed
    ;[1 1 1] Check for 'CanMoveL'
    (Physics|SetEnableGravity _sphere1 false))
  (:Released
    (Physics|SetEnableGravity _sphere1 true)
    (Physics|SetSimulatePhysics _sphere1 true)
    (Variables|Default|SetGrabbing_L false)))

(event Input|ActionEvents|InputActionLift_R_Action
  (params (Key :type Key%20Structure :default "None"))
  (bind _sphere (Variables|Default|GetSphere))
  (:Pressed
    ;[1 1 1] Check for 'CanMoveR'
    (Physics|SetEnableGravity _sphere false))
  (:Released
    (Physics|SetEnableGravity _sphere true)
    (Physics|SetSimulatePhysics _sphere true)
    (Variables|Default|SetGrabbing_R false)))

(event Input|AxisEvents|InputAxisLift_L
  (params (AxisValue :type Float%20%28single-precision%29))
  ;[1 1 1] Left Sphere Move
  (bind _output_get (Variables|Default|SetGrabbing_L (and (> AxisValue 0.0) (Variables|Default|GetisTouchingBar_L))))
  (if _output_get
    (Variables|Default|SetHasEverGrabbed true)
    (elif (or (Variables|Default|GetGrabbing_R) (not (Variables|Default|GetHasEverGrabbed)))
      (Physics|AddForce (Variables|Default|GetSphere1) "0, 0,500.000000" "None" true))))

(event Input|AxisEvents|InputAxisLift_R
  (params (AxisValue :type Float%20%28single-precision%29))
  ;[1 1 1] Right Sphere Move
  (bind _output_get (Variables|Default|SetGrabbing_R (and (> AxisValue 0.0) (Variables|Default|GetisTouchingBar_R))))
  (if (not _output_get)
    (if (Variables|Default|GetGrabbing_L)
      (Physics|AddForce (Variables|Default|GetSphere) "0, 0,500.000000" "None" true))))

(event Input|AxisEvents|InputAxisMoveForward
  (params (AxisValue :type Float%20%28single-precision%29))
  (bind _sphere1 (Variables|Default|GetSphere1))
  ;[1 1 1] Left Sphere Move
  (if (Variables|Default|GetGrabbing_L)
    (Physics|SetSimulatePhysics (Variables|Default|GetSphere1) false)
    (else
      (bind _output_get (Variables|Default|SetSphereL_Pos (Transformation|GetWorldLocation _sphere1)))
      (Transformation|SetWorldLocation _sphere1 (+ _output_get (* (Variables|Default|GetForwardSpeedVec) AxisValue)) false false))))

(event Input|AxisEvents|InputAxisMoveRight
  (params (AxisValue :type Float%20%28single-precision%29))
  (bind _sphere1 (Variables|Default|GetSphere1))
  ;[1 1 1] Left Sphere Move
  (if (Variables|Default|GetGrabbing_L)
    (Physics|SetSimulatePhysics (Variables|Default|GetSphere1) false)
    (else
      (bind _output_get (Variables|Default|SetSphereL_Pos (Transformation|GetWorldLocation _sphere1)))
      (Transformation|SetWorldLocation _sphere1 (+ _output_get (* (Variables|Default|GetRightSpeedVec) AxisValue)) false false))))

(event Input|AxisEvents|InputAxisMoveForward_R
  (params (AxisValue :type Float%20%28single-precision%29))
  (bind _sphere (Variables|Default|GetSphere))
  ;[1 1 1] Right Sphere Move
  (if (Variables|Default|GetGrabbing_R)
    (Physics|SetSimulatePhysics (Variables|Default|GetSphere) false)
    (else
      (bind _output_get (Variables|Default|SetSphere_R_Pos (Transformation|GetWorldLocation _sphere)))
      (Transformation|SetWorldLocation _sphere (+ _output_get (* (Variables|Default|GetForwardSpeedVec) AxisValue)) false false))))

(event Input|AxisEvents|InputAxisMoveRight_R
  (params (AxisValue :type Float%20%28single-precision%29))
  (bind _sphere (Variables|Default|GetSphere))
  ;[1 1 1] Right Sphere Move
  (if (Variables|Default|GetGrabbing_R)
    (Physics|SetSimulatePhysics (Variables|Default|GetSphere) false)
    (else
      (bind _output_get (Variables|Default|SetSphere_R_Pos (Transformation|GetWorldLocation _sphere)))
      (Transformation|SetWorldLocation _sphere (+ _output_get (* (Variables|Default|GetRightSpeedVec) AxisValue)) false false))))

(fn ConstructionScript)